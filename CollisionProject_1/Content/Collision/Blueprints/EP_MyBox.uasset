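; EP_MyBox is a collision test actor that reports contacts on its Cube2 component and acts as a trigger.
; Begin overlap, end overlap and hit events print the names of both components and the other actor, all using the same overlap label.
; Begin overlap also calls Play on every MoveRect entry, while its MoveLeftRight and RotationBall loops are empty.
; An unconnected pair of index-printing loops never runs.
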(event OnComponentBeginOverlap(Cube2)
  (params (OverlappedComponent :type Primitive%20Component%20Object%20Reference) (OtherActor :type Actor%20Object%20Reference) (OtherComp :type Primitive%20Component%20Object%20Reference) (OtherBodyIndex :type Integer) (bFromSweep :type Boolean) (SweepResult :type Hit%20Result%20Structure%20%28by%20ref%29))
  (Development|PrintString (Utilities|String|Append "Overlapped Component" (Utilities|GetDisplayName OverlappedComponent) "Other Actor" (Utilities|GetDisplayName OtherActor) "Other Component" (Utilities|GetDisplayName OtherComp)) true true "(R=0.000000,G=0.660000,B=1.000000,A=1.000000)" 2e+02)
  (Utilities|FlowControl|Sequence
    (:then_0
      (for _array_element (Variables|디폴트|GetMoveRect)
        (Class|LevelSequenceEditorBlueprintLibrary|Play)))
    (:then_1
      (for _array_element_2 (Variables|디폴트|GetMoveLeftRight)
        _))
    (:then_2
      (for _array_element_3 (Variables|디폴트|GetRotationBall)
        _))))

(event OnComponentEndOverlap(Cube2)
  (params (OverlappedComponent :type Primitive%20Component%20Object%20Reference) (OtherActor :type Actor%20Object%20Reference) (OtherComp :type Primitive%20Component%20Object%20Reference) (OtherBodyIndex :type Integer))
  (Development|PrintString (Utilities|String|Append "Overlapped Component" (Utilities|GetDisplayName OverlappedComponent) "Other Actor" (Utilities|GetDisplayName OtherActor) "Other Component" (Utilities|GetDisplayName OtherComp)) true true "(R=0.000000,G=0.660000,B=1.000000,A=1.000000)" 2e+02))

(event OnComponentHit(Cube2)
  (params (HitComponent :type Primitive%20Component%20Object%20Reference) (OtherActor :type Actor%20Object%20Reference) (OtherComp :type Primitive%20Component%20Object%20Reference) (NormalImpulse :type Vector :default "0, 0, 0") (Hit :type Hit%20Result%20Structure%20%28by%20ref%29))
  (Development|PrintString (Utilities|String|Append "Overlapped Component" (Utilities|GetDisplayName HitComponent) "Other Actor" (Utilities|GetDisplayName OtherActor) "Other Component" (Utilities|GetDisplayName OtherComp)) true true "(R=0.000000,G=0.660000,B=1.000000,A=1.000000)" 2e+02))

(fn ConstructionScript)