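; BP_MoveRect is an actor that moves its static mesh around a rectangular loop in the relative X-Z plane.
; The Play event starts a fast looping timer on Update_Move, which steps the mesh and switches the MoveType state at each position limit.
; R key press and release only print debug strings.
; Input enable/disable nodes and a boolean up-down mover are present but never run.
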(event Custom|Play
  (Utilities|Time|SetTimerbyFunctionName 0 "Update_Move" 0.01 true))

(event Collision|EventActorBeginOverlap
  (params (OtherActor :type Actor%20Object%20Reference)))

(event Input|KeyboardEvents|R
  (params (Key :type Key%20Structure :default "None"))
  (:Pressed
    (Development|PrintString "Pressed"))
  (:Released
    (Development|PrintString "UnPressed")))

(fn ConstructionScript)

(fn UpdateMove
  (bind _staticmesh (Variables|Default|GetStaticMesh))
  (switch Utilities|FlowControl|Switch|SwitchonEn_MoveType (Variables|Default|GetMoveType)
    (:NewEnumerator0
      (Transformation|AddRelativeLocation _staticmesh "10.000000,0.0,0.0" false false)
      (if (> (.x (Variables|/Script/Engine.SceneComponent|GetRelativeLocation (Variables|Default|GetStaticMesh))) 5e+02)
        (Variables|Default|SetMoveType "NewEnumerator1")))
    (:NewEnumerator1
      (Transformation|AddRelativeLocation _staticmesh "0.000000,0.000000,10.000000" false false)
      (if (> (.z (Variables|/Script/Engine.SceneComponent|GetRelativeLocation (Variables|Default|GetStaticMesh))) 5e+02)
        (Variables|Default|SetMoveType "NewEnumerator2")))
    (:NewEnumerator2
      (Transformation|AddRelativeLocation _staticmesh "-10.000000, 0,0.000000" false false)
      (if (<= (.x (Variables|/Script/Engine.SceneComponent|GetRelativeLocation (Variables|Default|GetStaticMesh))) -5e+02)
        (Variables|Default|SetMoveType "NewEnumerator3")))
    (:NewEnumerator3
      (Transformation|AddRelativeLocation _staticmesh "0.000000, 0,-10.000000" false false)
      (if (<= (.z (Variables|/Script/Engine.SceneComponent|GetRelativeLocation (Variables|Default|GetStaticMesh))) -5e+02)
        (Variables|Default|SetMoveType "NewEnumerator0")))))