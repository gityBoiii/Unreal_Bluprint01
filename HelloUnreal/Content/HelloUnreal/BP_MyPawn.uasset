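; A test player pawn that flies freely along the camera's view using axis inputs.
; MoveForward and MoveRight offset the actor along camera manager vectors scaled by Speed, without sweep, while look axes feed controller pitch and yaw.
; SpeedUp and SpeedDown step Speed within clamped limits and print it.
; Debug prints remain; the PrintTime elapsed minutes-and-seconds printer, using IntToStr00 zero-padding, is never run.
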(event EventBeginPlay
  (Development|PrintString (Utilities|GetDisplayName self) false false "(R=0.000000,G=0.660000,B=1.000000,A=1.000000)" 6e+01))

(event EventTick
  (params (DeltaSeconds :type Float%20%28single-precision%29)))

(event Input|ActionEvents|InputActionTestKey
  (params (Key :type Key%20Structure :default "None"))
  ;[1 1 1] 콘솔 출력
  (:Pressed
    (Development|PrintString "f"))
  (:Released
    (Development|PrintString "ff")))

(event Input|ActionEvents|InputActionSpeedUp
  (params (Key :type Key%20Structure :default "None"))
  ;[1 1 1] 속도 증감
  (:Pressed
    (bind _output_get (Variables|Default|SetSpeed (Math|Float|Clamp(Float) (+ (Variables|Default|GetSpeed) 1e+01) 1e+01 1e+02)))
    (Development|PrintString (Utilities|String|Append "증가 :" (Utilities|String|ToString(Float) _output_get)))))

(event Input|ActionEvents|InputActionSpeedDown
  (params (Key :type Key%20Structure :default "None"))
  ;[1 1 1] 속도 증감
  (:Pressed
    (bind _output_get (Variables|Default|SetSpeed (Math|Float|Clamp(Float) (+ (Variables|Default|GetSpeed) -1e+01) 1e+01 1e+02)))
    (Development|PrintString (Utilities|String|Append "감소 :" (Utilities|String|ToString(Float) _output_get)))))

(event Input|AxisEvents|InputAxisAxisTest
  (params (AxisValue :type Float%20%28single-precision%29))
  ;[1 1 1] 콘솔 출력
)

(event Input|AxisEvents|InputAxisMoveRight
  (params (AxisValue :type Float%20%28single-precision%29))
  ;[1 1 1] 캐릭 이동
  (Transformation|AddActorWorldOffset (* (Transformation|GetActorRightVector (Game|GetPlayerCameraManager 0)) (* AxisValue (Variables|Default|GetSpeed)))))

(event Input|AxisEvents|InputAxisLookUp
  (params (AxisValue :type Float%20%28single-precision%29))
  ;[1 1 1] 캐릭 이동
  (Pawn|Input|AddControllerPitchInput AxisValue))

(event Input|AxisEvents|InputAxisLookRight
  (params (AxisValue :type Float%20%28single-precision%29))
  ;[1 1 1] 캐릭 이동
  (Pawn|Input|AddControllerYawInput AxisValue))

(event Input|AxisEvents|InputAxisMoveForward
  (params (AxisValue :type Float%20%28single-precision%29))
  ;[1 1 1] 캐릭 이동
  (Transformation|AddActorWorldOffset (* (Transformation|GetActorForwardVector (Game|GetPlayerCameraManager 0)) (* AxisValue (Variables|Default|GetSpeed)))))

(fn ConstructionScript)

(fn InttoStr00
  (params (Number :type Float%20%28single-precision%29))
  (bind _returnvalue (Math|Float|Floor Number))
  (bind _returnvalue_2 (Utilities|String|ToString(Integer) _returnvalue))
  (if (< _returnvalue 10)
    (return (Utilities|String|Append "0" _returnvalue_2))
    (else
      (return _returnvalue_2))))

(fn PrintTime
  (params (DeltaSeconds :type Float%20%28single-precision%29))
  (bind _output_get (Variables|Default|SetTotalDeltaSeconds (+ (Variables|Default|GetTotalDeltaSeconds) DeltaSeconds)))
  (if (Utilities|Enum|NotEqual(Enum) (Utilities|String|Append (wontae|InttoStr00 (/ _output_get 6e+01)) "분" (wontae|InttoStr00 (Math|Float|%(Float) _output_get 6e+01)) "초") (Variables|Default|GetBeforeString))
    (Development|PrintString (Utilities|String|Append (wontae|InttoStr00 (/ _output_get 6e+01)) "분" (wontae|InttoStr00 (Math|Float|%(Float) _output_get 6e+01)) "초") true true "(R=0.000000,G=0.660000,B=1.000000,A=1.000000)" 1e+01)
    (Variables|Default|SetBeforeString (Utilities|String|Append (wontae|InttoStr00 (/ _output_get 6e+01)) "분" (wontae|InttoStr00 (Math|Float|%(Float) _output_get 6e+01)) "초"))))