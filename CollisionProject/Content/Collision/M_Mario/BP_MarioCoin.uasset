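; BP_MarioCoin is a spinning pickup coin that adds to the player's coin count.
; Tick increases the mesh's roll by a fixed, frame-rate-dependent step.
; Any CollisionBox overlap, without checking the other actor, disables mesh collision and plays a 2D sound.
; It then casts player pawn 0 to ThirdPersonCharacter, adds MarioCoin to its MarioCoins, destroys the coin and sets IsDestroyed.
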(event OnComponentBeginOverlap(CollisionBox)
  (params (OverlappedComponent :type Primitive%20Component%20Object%20Reference) (OtherActor :type Actor%20Object%20Reference) (OtherComp :type Primitive%20Component%20Object%20Reference) (OtherBodyIndex :type Integer) (bFromSweep :type Boolean) (SweepResult :type Hit%20Result%20Structure%20%28by%20ref%29))
  (Collision|SetCollisionEnabled (Variables|Default|GetMarioCoinMesh) "NoCollision")
  (Audio|PlaySound2D "/Engine/VREditor/Sounds/UI/Camera_Shutter.Camera_Shutter" 1.0 1.0 0.0 0 0)
  (bind _asthird_person_character (Utilities|Casting|CastToThirdPersonCharacter (Game|Player|GetPlayerPawn 0)))
  (Variables|/Game/ThirdPersonBP/Blueprints/ThirdPersonCharacter.ThirdPersonCharacter_C|SetMarioCoins _asthird_person_character (+ (Variables|/Game/ThirdPersonBP/Blueprints/ThirdPersonCharacter.ThirdPersonCharacter_C|GetMarioCoins _asthird_person_character) (Variables|Default|GetMarioCoin)))
  (Actor|DestroyActor)
  (Development|PrintString "Mario Coin Destroyed")
  (Variables|Default|SetIsDestroyed true))

(event EventBeginPlay)

(event Collision|EventActorBeginOverlap
  (params (OtherActor :type Actor%20Object%20Reference)))

(event EventTick
  (params (DeltaSeconds :type Float%20%28single-precision%29))
  (bind _mariocoinmesh (Variables|Default|GetMarioCoinMesh))
  (bind _relativerotation (Variables|/Script/Engine.SceneComponent|GetRelativeRotation _mariocoinmesh))
  (Transformation|SetRelativeRotation _mariocoinmesh (Math|Rotator|MakeRotator (+ (.roll _relativerotation) 2.0) (.pitch _relativerotation) (.yaw _relativerotation)) false false))

(fn ConstructionScript)