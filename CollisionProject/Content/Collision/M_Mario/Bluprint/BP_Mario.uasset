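; BP_Mario is a Mario Blueprint that holds the rule for earning a 1-up from collected coins.
; 1UpCoin scans the MarioCoins array and returns false at the first undestroyed coin, otherwise true, printing debug text either way.
; Play1upSound calls that check but ignores its result, so the 1-up sound always plays.
; The event graph and construction script are empty.
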(event EventBeginPlay)

(event Collision|EventActorBeginOverlap
  (params (OtherActor :type Actor%20Object%20Reference)))

(event EventTick
  (params (DeltaSeconds :type Float%20%28single-precision%29)))

(fn ConstructionScript)

(fn 1UpCoin
  (for (_array_element _array_index) (Variables|Default|GetMarioCoins)
    (if (not (Variables|/Game/Collision/M_Mario/Bluprint/BP_MarioCoin.BP_MarioCoin_C|GetIsDestroyed _array_element))
      (Development|PrintString (Utilities|String|Append "MarioCoin" (Utilities|String|ToString(Integer) _array_index) "!"))
      (return false)))
  (Development|PrintString (Utilities|String|Append "3Coins! " "1up"))
  (return true))

(fn Play1upSound
  (CallFunction|1UpCoin)
  (Audio|PlaySound2D "/Game/Collision/M_Mario/Sound/Mario_1Up.Mario_1Up" 1.0 1.0 0.0 0 0))