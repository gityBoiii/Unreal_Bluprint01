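; BP_MoveLeftRight is an actor whose static mesh slides back and forth along its local X axis while triggered by BP_MyBox actors.
; On BeginPlay it binds to every BP_MyBox's begin-overlap dispatcher and end-overlap event, which call Play and Stop.
; A timeline drives the relative X position, flipping IsMoveRight on finish to alternate Play and Reverse in a continuous loop until stopped.
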(event EventPlay
  (if (Variables|Default|GetIsMoveRight) :!label _label
    (bind _value (Timeline|타임라인_0 Play)
      (:Update
        (Transformation|SetRelativeLocation (Variables|Default|GetStaticMesh) (Math|Vector|MakeVector (* _value 1e+03) 0.0 0.0) false false))
      (:Finished
        (Variables|Default|SetIsMoveRight (not (Variables|Default|GetIsMoveRight)))
        (goto _label)))
    (else
      (Timeline|타임라인_0 Reverse))))

(event EventStop
  (bind _value (Timeline|타임라인_0 Stop)
    (:Update
      (Transformation|SetRelativeLocation (Variables|Default|GetStaticMesh) (Math|Vector|MakeVector (* _value 1e+03) 0.0 0.0) false false))
    (:Finished
      (Variables|Default|SetIsMoveRight (not (Variables|Default|GetIsMoveRight)))
      (if (Variables|Default|GetIsMoveRight)
        (Timeline|타임라인_0 Play)
        (else
          (Timeline|타임라인_0 Reverse))))))

(event EventBeginPlay
  ;[1 1 1] My Box 클래스의
  (bind _outactors (Actor|GetAllActorsOfClass "/Game/Collision/Blueprints/BP_MyBox.BP_MyBox_C"))
  ;[1 1 1] 오브젝트
  (for _array_element _outactors
    ;[1 1 1] 이벤트 디스패처에 바인딩
    (EventDispatchers|BindEventtoEventDispatcherBeginOverlap _array_element (EventDispatchers|CreateEvent :!event EventBeginOverlap))
    (Collision|BindEventtoOnActorEndOverlap _array_element (EventDispatchers|CreateEvent :!event EventEndOverlap))))

(fn ConstructionScript)

(fn EventBeginOverlap
  (params (bResult :type Boolean))
  (CallFunction|Play))

(fn EventEndOverlap
  (params (OverlappedActor :type Actor%20Object%20Reference) (OtherActor :type Actor%20Object%20Reference))
  (CallFunction|Stop))